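; BP_Turret is a stationary enemy that fires BP_Bullet projectiles at a regular interval.
; It fires on BeginPlay and on a looping FireRate timer, spawning bullets at ShootPoint and setting their velocity from the capsule's forward vector and bullet Speed.
; A player overlapping its Box has input disabled and Restart called.
; UpdateFlipbook and UpdateRotation are empty, so the turret does no animation or rotation updates there.
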(event OnComponentBeginOverlap(Box)
  (params (OverlappedComponent :type Primitive%20Component%20Object%20Reference) (OtherActor :type Actor%20Object%20Reference) (OtherComp :type Primitive%20Component%20Object%20Reference) (OtherBodyIndex :type Integer) (bFromSweep :type Boolean) (SweepResult :type Hit%20Result%20Structure%20%28by%20ref%29))
  (bind _asbp_player_base (Utilities|Casting|CastToBP_PlayerBase OtherActor))
  (Input|DisableInput _asbp_player_base (Game|GetPlayerController 0))
  (Default|Restart _asbp_player_base))

(event Custom|Fire
  (CallFunction|FireProjectile))

(event EventBeginPlay
  (Utilities|Time|SetTimerbyEvent (delegate Custom|Fire) (Variables|Default|GetFireRate) true)
  (CallFunction|FireProjectile))

(fn ConstructionScript
  (|CallParentFunction))

(fn UpdateFlipbook)

(fn UpdateRotation)

(fn FireProjectile
  (bind _returnvalue (Game|SpawnActorfromClass "/Game/Blueprints/Enemies/StationaryEnemies/BP_Bullet.BP_Bullet_C" (Math|Transform|MakeTransform (Transformation|GetWorldLocation (Variables|Default|GetShootPoint)) "0, 0, 0" "1,1,1") "Undefined" 0 0))
  (if (Utilities|IsValid _returnvalue)
    (Game|Components|ProjectileMovement|SetVelocityinLocalSpace (Variables|/Game/Blueprints/Enemies/StationaryEnemies/BP_Bullet.BP_Bullet_C|GetProjectileMovement _returnvalue) (* (Math|Vector|GetForwardVector (Transformation|GetWorldRotation (Variables|Default|GetCapsuleComponent self))) (Variables|/Game/Blueprints/Enemies/StationaryEnemies/BP_Bullet.BP_Bullet_C|GetSpeed _returnvalue)))))