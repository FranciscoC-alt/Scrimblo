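; BP_EnemyBase is an enemy base Blueprint that tracks health and death state.
; The construction script sets Health to DefaultHealth, and AnyDamage subtracts incoming damage, clamped between zero and that default.
; When Health reaches zero, IsDead is set once, while the EnemyDied function is empty and not called in these graphs.
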(event Game|Damage|EventAnyDamage
  (params (Damage :type Float%20%28single-precision%29) (DamageType :type Damage%20Type%20Object%20Reference) (InstigatedBy :type Controller%20Object%20Reference) (DamageCauser :type Actor%20Object%20Reference))
  (Variables|Default|SetHealth (Math|Float|Clamp(Float) (- (Variables|Default|GetHealth) Damage) 0.0 (Variables|Default|GetDefaultHealth)))
  (if (and (<= (Variables|Default|GetHealth) 0.0) (not (Variables|Default|GetIsDead)))
    (Variables|Default|SetIsDead true)))

(fn ConstructionScript
  (Variables|Default|SetHealth (Variables|Default|GetDefaultHealth)))

(fn EnemyDied)