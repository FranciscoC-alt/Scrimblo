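; BP_Button is a 2D Paper2D pressure-style button that toggles linked actors when a BP_PlayerBase overlaps it.
; Interact flips each BP_ActivateBase in ActivatedActors between Activate and Deactivate, then shows the pressed flipbook.
; When the player leaves and CanReset is set, Reset toggles the actors again and restores the unpressed flipbook, unless the first player pawn still overlaps the collider.
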(event EventBeginPlay
  (|CallParentFunction) ; This node is disabled and will not be called.\nDrag off pins to build functionality.
)

(event Collision|EventActorBeginOverlap
  (params (OtherActor :type Actor%20Object%20Reference))
  (bind _asbp_player_base (Utilities|Casting|CastToBP_PlayerBase OtherActor))
  (CallFunction|Interact _asbp_player_base))

(event Collision|EventActorEndOverlap
  (params (OtherActor :type Actor%20Object%20Reference))
  (Utilities|Casting|CastToBP_PlayerBase OtherActor)
  (if (Variables|Default|GetbCanReset)
    (CallFunction|Reset)))

(fn ConstructionScript
  (|CallParentFunction))

(fn Interact
  (params (PlayerRef :type BP%20Player%20Base%20Object%20Reference))
  (|CallParentFunction PlayerRef)
  (for _array_element (Variables|Default|GetActivatedActors)
    (bind _asbp_activate_base (Utilities|Casting|CastToBP_ActivateBase _array_element))
    (if (Variables|/Game/Blueprints/Activate/BP_ActivateBase.BP_ActivateBase_C|GetActivated _asbp_activate_base)
      (Default|Deactivate _asbp_activate_base)
      (Variables|/Game/Blueprints/Activate/BP_ActivateBase.BP_ActivateBase_C|SetActivated _asbp_activate_base false)
      (else
        (Default|Activate _asbp_activate_base)
        (Variables|/Game/Blueprints/Activate/BP_ActivateBase.BP_ActivateBase_C|SetActivated _asbp_activate_base true))))
  (Sprite|SetFlipbook (Variables|Default|GetPaperFlipbook) "/Game/Assets/Flipbooks/Interactables/Buttons/FB_RedButtonPressed.FB_RedButtonPressed"))

(fn Reset
  (if (not (Collision|IsOverlappingActor (Variables|Default|GetInteractive%20Collider) (Game|Player|GetPlayerPawn 0) :!class /Script/Engine.PrimitiveComponent))
    (for _array_element (Variables|Default|GetActivatedActors)
      (bind _asbp_activate_base (Utilities|Casting|CastToBP_ActivateBase _array_element))
      (if (Variables|/Game/Blueprints/Activate/BP_ActivateBase.BP_ActivateBase_C|GetActivated _asbp_activate_base)
        (Default|Deactivate _asbp_activate_base)
        (Variables|/Game/Blueprints/Activate/BP_ActivateBase.BP_ActivateBase_C|SetActivated _asbp_activate_base false)
        (else
          (Default|Activate _asbp_activate_base)
          (Variables|/Game/Blueprints/Activate/BP_ActivateBase.BP_ActivateBase_C|SetActivated _asbp_activate_base true))))
    (Sprite|SetFlipbook (Variables|Default|GetPaperFlipbook) "/Game/Assets/Flipbooks/Interactables/Buttons/FB_RedButton.FB_RedButton")))