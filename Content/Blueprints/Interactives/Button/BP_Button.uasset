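; BP_Button is an interactive Paper2D button that toggles the actors listed in its ActivatedActors array.
; Interact flips each BP_ActivateBase actor between Activate and Deactivate, updates its Activated flag, then shows the red pressed flipbook.
; Reset repeats the toggle, restores the unpressed red flipbook and makes a timer call naming itself.
; UpdateFlipbook is an empty stub, and the button color selection is unused.
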(event EventBeginPlay
  (|CallParentFunction) ; This node is disabled and will not be called.\nDrag off pins to build functionality.
)

(fn ConstructionScript
  (|CallParentFunction))

(fn Interact
  (params (PlayerRef :type BP%20Player%20Base%20Object%20Reference))
  (|CallParentFunction PlayerRef)
  (for _array_element (Variables|Default|GetActivatedActors)
    (bind _asbp_activate_base (Utilities|Casting|CastToBP_ActivateBase _array_element))
    (if (Variables|/Game/Blueprints/Activate/BP_ActivateBase.BP_ActivateBase_C|GetActivated _asbp_activate_base)
      (Default|Deactivate _asbp_activate_base)
      (Variables|/Game/Blueprints/Activate/BP_ActivateBase.BP_ActivateBase_C|SetActivated _asbp_activate_base false)
      (else
        (Default|Activate _asbp_activate_base)
        (Variables|/Game/Blueprints/Activate/BP_ActivateBase.BP_ActivateBase_C|SetActivated _asbp_activate_base true))))
  (Sprite|SetFlipbook (Variables|Default|GetPaperFlipbook) "/Game/Assets/Flipbooks/Interactables/Buttons/FB_RedButtonPressed.FB_RedButtonPressed"))

(fn Reset
  (for _array_element (Variables|Default|GetActivatedActors)
    (bind _asbp_activate_base (Utilities|Casting|CastToBP_ActivateBase _array_element))
    (if (Variables|/Game/Blueprints/Activate/BP_ActivateBase.BP_ActivateBase_C|GetActivated _asbp_activate_base)
      (Default|Deactivate _asbp_activate_base)
      (Variables|/Game/Blueprints/Activate/BP_ActivateBase.BP_ActivateBase_C|SetActivated _asbp_activate_base false)
      (else
        (Default|Activate _asbp_activate_base)
        (Variables|/Game/Blueprints/Activate/BP_ActivateBase.BP_ActivateBase_C|SetActivated _asbp_activate_base true))))
  (Sprite|SetFlipbook (Variables|Default|GetPaperFlipbook) "/Game/Assets/Flipbooks/Interactables/Buttons/FB_RedButton.FB_RedButton")
  (Utilities|Time|SetTimerbyFunctionName 0 "Reset" 0.0))

(fn UpdateFlipbook
  (if (Variables|Default|GetIsPressed)
    _))