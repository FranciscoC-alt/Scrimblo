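; BP_SkrunklyCage is a trigger actor that shows a restart screen when the player enters its box.
; It creates the WPB_Restart widget at BeginPlay with Level1 as the restart point.
; When the player pawn overlaps the box, it adds the widget to the viewport, switches to UI-only input with a visible cursor, and disables pawn input.
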(event OnComponentBeginOverlap(Box)
  (params (OverlappedComponent :type Primitive%20Component%20Object%20Reference) (OtherActor :type Actor%20Object%20Reference) (OtherComp :type Primitive%20Component%20Object%20Reference) (OtherBodyIndex :type Integer) (bFromSweep :type Boolean) (SweepResult :type Hit%20Result%20Structure%20%28by%20ref%29))
  (if (== OtherActor (Game|Player|GetPlayerPawn 0))
    (UserInterface|Viewport|AddtoViewport (Variables|Default|GetRestartWidget) 0)
    (Input|SetInputModeUIOnly (Game|GetPlayerController 0) 0 "DoNotLock")
    (Variables|/Script/Engine.PlayerController|SetbShowMouseCursor (Game|GetPlayerController 0) true)
    (Input|DisableInput (Game|Player|GetPlayerPawn 0) (Game|GetPlayerController 0))))

(event EventBeginPlay
  (bind _returnvalue (UserInterface|CreateWidget "/Game/Widgets/WPB_Restart.WPB_Restart_C" 0 "Level1"))
  (Variables|Default|SetRestartWidget _returnvalue))

(fn ConstructionScript)